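; Boss actor that handles taking damage and its death sequence.
; AnyDamage passes a DoOnce gate that resets only after the hit-react montage and red material tint finish, so hits during the reaction are ignored.
; At zero health it stays red while a timeline scales it, triggering camera shake and flare spawns on every update.
; A delayed poof explosion and DestroyActor follow, with explosion cleanup queued after the boss's own destruction.
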(event Game|Damage|EventAnyDamage
  (params (Damage :type Float%20%28single-precision%29) (DamageType :type Damage%20Type%20Object%20Reference) (InstigatedBy :type Controller%20Object%20Reference) (DamageCauser :type Actor%20Object%20Reference))
  (bind _mesh (Variables|Character|GetMesh))
  (bind _mesh_2 (Variables|Character|GetMesh))
  (Utilities|FlowControl|DoOnce false :!label _label
    (:Completed
      (bind _output_get (Variables|Stats|SetHealth (- (Variables|Stats|GetHealth) Damage)))
      (if (<= _output_get 0.0)
        (bind _returnvalue (Rendering|Material|CreateDynamicMaterialInstance _mesh_2 0 "/Game/Characters/Mannequins/Materials/Instances/Manny/MI_Manny_01.MI_Manny_01" "None" :!class /Script/Engine.PrimitiveComponent))
        (Rendering|Material|SetVectorParameterValue _returnvalue "Tint" "(R=1.000000,G=0.006161,B=0.000000,A=1.000000)" :!class /Script/Engine.MaterialInstanceDynamic)
        (bind _returnvalue_2 (Rendering|Material|CreateDynamicMaterialInstance _mesh_2 1 "/Game/Characters/Mannequins/Materials/Instances/Manny/MI_Manny_02.MI_Manny_02" "None" :!class /Script/Engine.PrimitiveComponent))
        (Rendering|Material|SetVectorParameterValue _returnvalue_2 "Tint" "(R=1.000000,G=0.006161,B=0.000000,A=1.000000)" :!class /Script/Engine.MaterialInstanceDynamic)
        (bind _size_track (Timeline|Boss_Grownth Play)
          (:Update
            (Transformation|SetActorScale3D _size_track)
            (Camera|PlayWorldCameraShake "/Game/Blueprints/BP_CameraShake.BP_CameraShake_C" (Transformation|GetActorLocation) 0.0 5e+03 1.0 true)
            (Game|SpawnActorfromClass "/Game/Blueprints/BP_Boss_Flares.BP_Boss_Flares_C" (Transformation|GetActorTransform) "Undefined" 0 0)
            (Utilities|FlowControl|Delay 3.0)
            (bind _returnvalue_3 (Game|SpawnActorfromClass "/Game/Blueprints/BP_Poof_Explosion.BP_Poof_Explosion_C" (Transformation|GetActorTransform) "Undefined" 0 0))
            (Actor|DestroyActor)
            (Utilities|FlowControl|Delay 2.0)
            (Actor|DestroyActor _returnvalue_3)))
        (else
          (bind _returnvalue_4 (Rendering|Material|CreateDynamicMaterialInstance _mesh 0 "/Game/Characters/Mannequins/Materials/Instances/Manny/MI_Manny_01.MI_Manny_01" "None" :!class /Script/Engine.PrimitiveComponent))
          (Rendering|Material|SetVectorParameterValue _returnvalue_4 "Tint" "(R=1.000000,G=0.006161,B=0.000000,A=1.000000)" :!class /Script/Engine.MaterialInstanceDynamic)
          (bind _returnvalue_5 (Rendering|Material|CreateDynamicMaterialInstance _mesh 1 "/Game/Characters/Mannequins/Materials/Instances/Manny/MI_Manny_02.MI_Manny_02" "None" :!class /Script/Engine.PrimitiveComponent))
          (Rendering|Material|SetVectorParameterValue _returnvalue_5 "Tint" "(R=1.000000,G=0.006161,B=0.000000,A=1.000000)" :!class /Script/Engine.MaterialInstanceDynamic)
          (bind _returnvalue_6 (Animation|PlayAnimMontage "/Game/Animations/HitReact_Montage.HitReact_Montage" 1.0 "None"))
          (Utilities|FlowControl|Delay _returnvalue_6)
          (Rendering|Material|SetVectorParameterValue _returnvalue_4 "Tint" "(R=1.000000,G=1.000000,B=1.000000,A=0.000000)" :!class /Script/Engine.MaterialInstanceDynamic)
          (Rendering|Material|SetVectorParameterValue _returnvalue_5 "Tint" "(R=1.000000,G=1.000000,B=1.000000,A=0.000000)" :!class /Script/Engine.MaterialInstanceDynamic)
          (goto _label Reset))))))

(fn ConstructionScript)