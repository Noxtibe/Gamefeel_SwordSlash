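; BP_Trainer is a damageable character that reacts to hits and is destroyed when its Health runs out.
; AnyDamage passes through a DoOnce that resets after the hit reaction, so damage during a reaction is ignored.
; A surviving hit launches it along the mesh's negative right vector and tints two dynamic materials red while the HitReact montage plays.
; A lethal hit plays the death montage, waits its length, then destroys the actor.
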(event Game|Damage|EventAnyDamage
  (params (Damage :type Float%20%28single-precision%29) (DamageType :type Damage%20Type%20Object%20Reference) (InstigatedBy :type Controller%20Object%20Reference) (DamageCauser :type Actor%20Object%20Reference))
  (bind _mesh (Variables|Character|GetMesh))
  (Utilities|FlowControl|DoOnce false :!label _label
    (:Completed
      (bind _output_get (Variables|Stats|SetHealth (- (Variables|Stats|GetHealth) Damage)))
      (if (<= _output_get 0.0)
        (bind _returnvalue (Animation|PlayAnimMontage "/Game/Animations/Death_Montage.Death_Montage" 1.0 "None"))
        (Utilities|FlowControl|Delay _returnvalue)
        (Actor|DestroyActor)
        (else
          (Character|LaunchCharacter (* (Math|Vector|GetRightVector (Variables|Character|GetMesh)) -5e+02) false false)
          (bind _returnvalue_2 (Rendering|Material|CreateDynamicMaterialInstance _mesh 0 "/Game/Characters/Mannequins/Materials/Instances/Manny/MI_Manny_01.MI_Manny_01" "None" :!class /Script/Engine.PrimitiveComponent))
          (Rendering|Material|SetVectorParameterValue _returnvalue_2 "Tint" "(R=1.000000,G=0.006161,B=0.000000,A=1.000000)" :!class /Script/Engine.MaterialInstanceDynamic)
          (bind _returnvalue_3 (Rendering|Material|CreateDynamicMaterialInstance _mesh 1 "/Game/Characters/Mannequins/Materials/Instances/Manny/MI_Manny_02.MI_Manny_02" "None" :!class /Script/Engine.PrimitiveComponent))
          (Rendering|Material|SetVectorParameterValue _returnvalue_3 "Tint" "(R=1.000000,G=0.006161,B=0.000000,A=1.000000)" :!class /Script/Engine.MaterialInstanceDynamic)
          (bind _returnvalue_4 (Animation|PlayAnimMontage "/Game/Animations/HitReact_Montage.HitReact_Montage" 1.0 "None"))
          (Utilities|FlowControl|Delay _returnvalue_4)
          (Rendering|Material|SetVectorParameterValue _returnvalue_2 "Tint" "(R=1.000000,G=1.000000,B=1.000000,A=0.000000)" :!class /Script/Engine.MaterialInstanceDynamic)
          (Rendering|Material|SetVectorParameterValue _returnvalue_3 "Tint" "(R=1.000000,G=1.000000,B=1.000000,A=0.000000)" :!class /Script/Engine.MaterialInstanceDynamic)
          (goto _label Reset))))))

(fn ConstructionScript)